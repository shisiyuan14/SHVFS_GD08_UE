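; Round-based enemy spawner for crowd AI that spawns groups of BP_EnemyCharacter and calls RoundsFinish when rounds run out.
; A Delay-throttled Tick prunes dead entries from SpawnedEnemy, then sets IsAllDead once it is empty.
; While IsAllDead holds, it decrements Rounds and runs GoblinFactory; nothing here clears that flag.
; GoblinFactory line-traces for ground and spawns at random navigable points within Radius, leaving debug drawing on.
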(event `self.ReceiveBeginPlay`
  (if (> (`self.Rounds`) 1)
    _))

(event `self.ReceiveTick`
  (params (DeltaSeconds :type "Float (single-precision)"))
  (bind _spawnedenemy (`self.SpawnedEnemy`))
  (bind _rounds (`self.Rounds`))
  (`KismetSystemLibrary.Delay` 0.2)
  (if (`self.IsAllDead`)
    (if (> _rounds 0)
      (bind _result (`/Engine/EditorBlueprintResources/StandardMacros.DecrementInt` _rounds)
        (:`  `
          (set `self.Rounds` _result)
          (`self.Goblin Factory`)))
      (else
        (`self.RoundsFinish`)))
    (elif (> (`KismetArrayLibrary.Array_Length` _spawnedenemy) 0)
      (for _array_element _spawnedenemy
        (if (not (`/Game/Blueprint/Character/BP_ThirPersonCharacter.IsAlive` _array_element))
          (`KismetArrayLibrary.Array_RemoveItem` _spawnedenemy _array_element)))
      (else
        (set `self.IsAllDead` true)))))

(fn `Goblin Factory`
  (bind _returnvalue (`self.K2_GetActorLocation`))
  (bind (_returnvalue_location _returnvalue_rotation _returnvalue_scale) (`KismetMathLibrary.BreakTransform` (`self.GetTransform`)))
  (bind _num (`self.Num`))
  (if (> _num 0)
    (for _ (range _num)
      (bind (_outhit _returnvalue_2) (`KismetSystemLibrary.LineTraceSingleForObjects` :`Start` (+ _returnvalue (0.0 0.0 1000.0)) :`End` (+ _returnvalue (0.0 0.0 -1000.0)) :`ObjectTypes` (`|MakeArray` "ObjectTypeQuery2" "ObjectTypeQuery1" :!type "EObjectTypeQuery Enum") :`DrawDebugType` "Persistent"))
      (if _returnvalue_2
        (bind _randomlocation (`NavigationSystemV1.K2_GetRandomLocationInNavigableRadius` (`.Location` (`GameplayStatics.BreakHitResult` _outhit)) (`self.Radius`) null null))
        (`KismetSystemLibrary.DrawDebugSphere` _randomlocation 100.0 4 (struct :`G` 1.0 :`B` 0.107318 :`A` 1.0) 5.0 2.0)
        (bind _returnvalue_3 (`|SpawnActorFromClass` (`self.EnemyClass`) (`KismetMathLibrary.MakeTransform` _randomlocation _returnvalue_rotation _returnvalue_scale) "Undefined" "OverrideRootScale" self null))
        (bind _asbp_enemy_character (cast `/Game/Blueprint/Character/BP_EnemyCharacter` _returnvalue_3))
        (`KismetArrayLibrary.Array_Add` (`self.SpawnedEnemy`) _asbp_enemy_character)))))

(fn `UserConstructionScript`)