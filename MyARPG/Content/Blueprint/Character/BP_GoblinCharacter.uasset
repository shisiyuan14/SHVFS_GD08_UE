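; Goblin enemy character, built on a parent class that supplies damage handling, with an attached weapon and a montage-based melee attack.
; On BeginPlay it spawns BP_GoblinWeapon and attaches it to the right weapon socket.
; When damaged it turns to face the damage causer, then runs the parent handling.
; DoMeleeAttack plays the attack montage behind melee-state checks, but its AI chase-then-attack caller is disconnected and never runs.
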(event `self.ReceiveBeginPlay`
  (`self.GetWeapon`))

(event `self.OnDamaged`
  (params (Damage :type "Float (single-precision)") (HitInfo :type "HitResult Structure (by ref)") (InstigatedCharacter :type "Character Object Reference") (DamageCauser :type "Actor Object Reference"))
  (bind (_returnvalue_roll _returnvalue_pitch _returnvalue_yaw) (`KismetMathLibrary.BreakRotator` (`KismetMathLibrary.FindLookAtRotation` (`self.K2_GetActorLocation`) (`self.K2_GetActorLocation` DamageCauser))))
  (`self.K2_SetActorRotation` (`KismetMathLibrary.MakeRotator` _returnvalue_roll 0.0 _returnvalue_yaw))
  (`parent.OnDamaged` Damage HitInfo InstigatedCharacter DamageCauser))

(event `self.ReceiveTick`
  (params (DeltaSeconds :type "Float (single-precision)"))
  (`parent.ReceiveTick` DeltaSeconds))

(fn `Do Melee Attack`
  (bind _returnvalue (`SkeletalMeshComponent.GetAnimInstance` (`self.Mesh`)))
  (if (`self.IsMelee`)
    (if (not (`AnimInstance.IsAnyMontagePlaying` _returnvalue))
      (`AnimInstance.Montage_Play` _returnvalue "/Game/Animations/NPC/AM_Guardian_Attack.AM_Guardian_Attack" 1.0 "MontageLength" 0.0 true :!label _label))
    (elif (not (> (`self.MeleeIndex`) 0))
      (goto _label))))

(fn `GetWeapon`
  (`self.GoblinWeapon`
    (:`then`)
    (:`else`
      (bind _returnvalue (`|SpawnActorFromClass` "/Game/Blueprint/Weapon/BP_GoblinWeapon.BP_GoblinWeapon_C" (`KismetMathLibrary.MakeTransform` (0.0 0.0 0.0)) "Undefined" "OverrideRootScale" self null))
      (bind _output_get (set `self.GoblinWeapon` _returnvalue))
      (bind _output_get_2 (set `self.CurrentWeapon` _output_get))
      (`self.SetOwner` _output_get_2 self)
      (`self.K2_AttachToComponent` _output_get_2 (`self.Mesh`) "b_MF_Weapon_RSocket" "SnapToTarget" "SnapToTarget" "KeepRelative" true))))

(fn `UserConstructionScript`
  (`parent.UserConstructionScript`))