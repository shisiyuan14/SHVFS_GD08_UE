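; Goblin enemy character that uses PawnSensing to detect, chase and melee the player.
; While alive, a Delay-throttled Tick runs AIMoveTo on player pawn 0, attacking on success if a target is held.
; Without a target it still moves toward that pawn, with GetNextNavPoint wired to the move results.
; Sight sets the target, lost line of sight clears it, and loud noises set a new destination.
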(event `self.ReceiveBeginPlay`
  (`parent.ReceiveBeginPlay`))

(event `self.ReceiveTick`
  (params (DeltaSeconds :type "Float (single-precision)"))
  (bind _targetpawn (`self.TargetPawn`))
  (`parent.ReceiveTick` DeltaSeconds)
  (if (`self.IsAlive`)
    (`KismetSystemLibrary.Delay` 1.5)
    (`|ExecutionSequence`
      (:`then_0`
        (`/Engine/EditorBlueprintResources/StandardMacros.IsValid` (`self.TargetPawn`)
          (:`Is Valid`
            (`|AIMoveTo` self (0.0 0.0 0.0) (`GameplayStatics.GetPlayerPawn` 0) 30.0 true
              (:`OnSuccess`
                (`self.Do Melee Attack`))))
          (:`Is Not Valid`
            (bind _movementresult (`|AIMoveTo` self (0.0 0.0 0.0) (`GameplayStatics.GetPlayerPawn` 0) 30.0 true)
              (:`then`
                (switch `EPathFollowingResult` _movementresult
                  (:`Success`
                    _)
                  (:`Aborted`
                    (`KismetSystemLibrary.Delay` 1.0)
                    (switch `EPathFollowingResult` _movementresult
                      (:`Aborted`
                        _))))
                (`self.GetNextNavPoint`))))))
      (:`then_1`
        (`/Engine/EditorBlueprintResources/StandardMacros.IsValid` _targetpawn
          (:`Is Valid`
            (if (not (`MyPawnSensingComponent.HasLineOfSightTo` (`self.MyPawnSensing_0`) _targetpawn))
              (set `self.TargetPawn` null))))))))

(event `self.MyPawnSensing_0.OnSeePawn`
  (params (Pawn :type "Pawn Object Reference"))
  (set `self.TargetPawn` Pawn))

(event `self.MyPawnSensing_0.OnHearNoise`
  (params (Instigator :type "Pawn Object Reference") (Location :type "Vector Structure (by ref)") (Volume :type "Float (single-precision)"))
  (if (> Volume 300.0)
    (`self.Set Enemy Destination` Location (`self.NoiseColor`))))

(fn `UserConstructionScript`
  (`parent.UserConstructionScript`))