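; Third-person player character with sprint, switchable hatchet and great blade weapons, and montage-driven melee combos.
; Weapon inputs destroy the other weapon, then spawn and attach the chosen one to the right-hand socket, or remove both to go unarmed.
; NormalAttack picks a montage by held weapon and calls DoMeleeAttack.
; That function starts the montage or, while IsMelee is set, jumps to sections listed by JumpSectionNotify to chain combos.
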(event `self.ReceiveBeginPlay`)

(event `InputAction|NormalAttack`
  (params (Key :type "Key Structure"))
  ;[1 1 1] Combo 2
  (:`Pressed`
    (`/Engine/EditorBlueprintResources/StandardMacros.IsValid` (`self.Hatchet02`)
      (:`Is Valid`
        (set `self.AttackMontage` "/Game/Characters/Animations/AM_Attack_Hammer.AM_Attack_Hammer"))
      (:`Is Not Valid`
        (`/Engine/EditorBlueprintResources/StandardMacros.IsValid` (`self.GreatBlade`)
          (:`Is Valid`
            (set `self.AttackMontage` "/Game/Characters/Animations/AM_Attack_Sword.AM_Attack_Sword"))
          (:`Is Not Valid`
            (set `self.AttackMontage` "/Game/Characters/Animations/AM_NormalAttack.AM_NormalAttack")))))
    (`self.Do Melee Attack`)))

(event `InputAction|Acceleration`
  (params (Key :type "Key Structure"))
  (bind _charactermovement (`self.CharacterMovement`))
  ;[1 1 1] Movement
  (:`Pressed`
    (set `CharacterMovementComponent.MaxWalkSpeed` 600.0 _charactermovement))
  (:`Released`
    (set `CharacterMovementComponent.MaxWalkSpeed` 300.0 _charactermovement)))

(event `InputAction|Weapon1`
  (params (Key :type "Key Structure"))
  ;[1 1 1] Weapon Switch
  (:`Pressed`
    (`self.K2_DestroyActor` (`self.GreatBlade`))
    (`self.TakeHatchet02`)))

(event `InputAction|Weapon2`
  (params (Key :type "Key Structure"))
  ;[1 1 1] Weapon Switch
  (:`Pressed`
    (`self.K2_DestroyActor` (`self.Hatchet02`))
    (`self.TakeGreatBlade`)))

(event `InputAction|Weapon3`
  (params (Key :type "Key Structure"))
  ;[1 1 1] Weapon Switch
  (:`Pressed`
    (`self.K2_DestroyActor` (`self.Hatchet02`))
    (`self.K2_DestroyActor` (`self.GreatBlade`))))

(fn `Do Melee Attack`
  (bind _returnvalue (`SkeletalMeshComponent.GetAnimInstance` (`self.Mesh`)))
  (if (`self.IsMelee`)
    (`self.Jump Section for Combo`)
    (if (not (`AnimInstance.IsAnyMontagePlaying` _returnvalue))
      (`AnimInstance.Montage_Play` _returnvalue (`self.AttackMontage`) 1.0 "MontageLength" 0.0 true :!label _label)
      (set `self.MeleeIndex` 1)
      (set `self.IsMelee` true))
    (elif (not (> (`self.MeleeIndex`) 0))
      (goto _label))))

(fn `IsAlive`
  (returns (IsTrue :type Boolean))
  (return true))

(fn `Jump Section for Combo`
  (bind _jumpsectionnotify (`self.JumpSectionNotify`))
  (`/Engine/EditorBlueprintResources/StandardMacros.IsValid` _jumpsectionnotify
    (:`Is Valid`
      (for _array_element (`/Game/Blueprint/AnimNotifies/JumpSectionNs.JumpSections` _jumpsectionnotify)
        (`AnimInstance.Montage_JumpToSection` (`SkeletalMeshComponent.GetAnimInstance` (`self.Mesh`)) _array_element (`self.AttackMontage`))))))

(fn `TakeGreatBlade`
  (`self.GreatBlade`
    (:`then`
      _)
    (:`else`
      (bind _returnvalue (`|SpawnActorFromClass` "/Game/Weapons/Blade_GreatBlade/BP_GreateBlade.BP_GreateBlade_C" (`KismetMathLibrary.MakeTransform` (0.0 0.0 0.0)) "Undefined" "OverrideRootScale" self null))
      (bind _output_get (set `self.GreatBlade` _returnvalue))
      (`self.SetOwner` _output_get self)))
  (`self.K2_AttachToComponent` _output_get (`self.Mesh`) "hand_rSocket" "SnapToTarget" "SnapToTarget" "KeepRelative" true))

(fn `TakeHatchet02`
  (`self.Hatchet02`
    (:`then`
      _)
    (:`else`
      (bind _returnvalue (`|SpawnActorFromClass` "/Game/Weapons/Blade_Hatchet02/BP_Hatchet02.BP_Hatchet02_C" (`KismetMathLibrary.MakeTransform` (0.0 0.0 0.0)) "Undefined" "OverrideRootScale" self null))
      (bind _output_get (set `self.Hatchet02` _returnvalue))
      (`self.SetOwner` _output_get self)))
  (`self.K2_AttachToComponent` _output_get (`self.Mesh`) "hand_rSocket" "SnapToTarget" "SnapToTarget" "KeepRelative" true))

(fn `UserConstructionScript`)