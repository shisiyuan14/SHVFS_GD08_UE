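; WeaponAttackNs is an animation notify state that marks the attack window of the character's weapon during an animation.
; On begin, it gets the current weapon from the owning BP_ThirPersonCharacter, sets IsAttacking and passes the notify's BaseDamage to BeginWeaponAttack.
; On end, it calls EndWeaponAttack on the current weapon.
; Both events act only when that weapon is valid.
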(fn `Received_NotifyBegin`
  (params (MeshComp :type "SkeletalMeshComponent Object Reference") (Animation :type "AnimSequenceBase Object Reference") (TotalDuration :type "Float (single-precision)") (EventReference :type "AnimNotifyEventReference Structure (by ref)"))
  (returns (ReturnValue :type Boolean))
  (bind _currentweapon (`/Game/Blueprint/Character/BP_ThirPersonCharacter.CurrentWeapon` (cast `/Game/Blueprint/Character/BP_ThirPersonCharacter` (`ActorComponent.GetOwner` MeshComp) :!pure true)))
  (`/Engine/EditorBlueprintResources/StandardMacros.IsValid` _currentweapon
    (:`Is Valid`
      (set `/Game/Blueprint/Weapon/BP_WeaponActor.IsAttacking` true _currentweapon)
      (`/Game/Blueprint/Weapon/BP_WeaponActor.BeginWeaponAttack` _currentweapon (`self.Base Damage`))
      (return true))))

(fn `Received_NotifyEnd`
  (params (MeshComp :type "SkeletalMeshComponent Object Reference") (Animation :type "AnimSequenceBase Object Reference") (EventReference :type "AnimNotifyEventReference Structure (by ref)"))
  (returns (ReturnValue :type Boolean))
  (bind _currentweapon (`/Game/Blueprint/Character/BP_ThirPersonCharacter.CurrentWeapon` (cast `/Game/Blueprint/Character/BP_ThirPersonCharacter` (`ActorComponent.GetOwner` MeshComp) :!pure true)))
  (`/Engine/EditorBlueprintResources/StandardMacros.IsValid` _currentweapon
    (:`Is Valid`
      (`/Game/Blueprint/Weapon/BP_WeaponActor.EndWeaponAttack` _currentweapon)
      (return false))))